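; AI controller that moves the player pawn in the Pacman game along a path of Targets actors, which this graph does not fill.
; Once the path is non-empty, Tick starts at the last array index and steps down to zero, hiding each reached node except that last-index one.
; Movement sets location by lerping from the current position with an alpha growing over time since the previous node, and rotates to face the target.
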(event EventTick
  (params (DeltaSeconds :type Float%20%28single-precision%29))
  (if (CallFunction|IsReadytoMove)
    (Utilities|FlowControl|Sequence
      (:then_0
        (Utilities|FlowControl|DoOnce false
          (:Completed
            (Variables|Default|SetCurrentTarget (- (Utilities|Array|Length (Variables|Default|GetTargets)) 1)))))
      (:then_1
        (Variables|Default|SetDeltatimeAccumulate (+ DeltaSeconds (Variables|Default|GetDeltatimeAccumulate)))
        (if (CallFunction|HasReachedTarget)
          (if (> (Variables|Default|GetCurrentTarget) 0)
            (Math|Integer|DecrementInt (Variables|Default|GetCurrentTarget)
              (:%20%20
                (Variables|Default|SetDeltatimeAccumulate 0.0)
                (CallFunction|MovetoTarget false :!label _label))))
          (else
            (goto _label)))))))

(fn ConstructionScript)

(fn IsReadytoMove
  (bind _targets (Variables|Default|GetTargets))
  (bind _returnvalue (Utilities|Array|Length _targets))
  (if (> _returnvalue 0)
    (Development|PrintString (Utilities|String|Append "PATH CONTAINS " (Utilities|String|ToString(Integer) _returnvalue) " NODES") false true "(R=0.000000,G=0.660000,B=1.000000,A=1.000000)" 0.0)
    (return true)
    (else
      (return false))))

(fn HasReachedTarget
  (if (Math|Vector|Equal(Vector) (Transformation|GetActorLocation (Pawn|GetControlledPawn)) (Transformation|GetActorLocation (Utilities|Array|Get(acopy) (Variables|Default|GetTargets) (Variables|Default|GetCurrentTarget))) (Variables|Default|GetAccuracy))
    (CallFunction|HideTarget)
    (return true)
    (else
      (return false))))

(fn MovetoTarget
  (params (Delta :type Boolean))
  (bind _returnvalue (Pawn|GetControlledPawn))
  (bind _targets (Variables|Default|GetTargets))
  (bind _currenttarget (Variables|Default|GetCurrentTarget))
  (bind _deltatimeaccumulate (Variables|Default|GetDeltatimeAccumulate))
  (bind _speed (Variables|Default|GetSpeed))
  (bind _returnvalue_2 (Transformation|GetActorLocation _returnvalue))
  (bind _returnvalue_3 (* _speed _deltatimeaccumulate))
  (bind _output (Utilities|Array|Get(acopy) _targets _currenttarget))
  (bind _returnvalue_4 (Transformation|GetActorLocation _output))
  (bind _returnvalue_5 (Math|Vector|Lerp(Vector) _returnvalue_2 _returnvalue_4 _returnvalue_3))
  (Transformation|SetActorLocation _returnvalue _returnvalue_5 false false)
  (Transformation|SetActorRotation _returnvalue (Math|Rotator|FindLookatRotation _returnvalue_5 _returnvalue_4)))

(fn HideTarget
  (bind _targets (Variables|Default|GetTargets))
  (bind _currenttarget (Variables|Default|GetCurrentTarget))
  (if (!= _currenttarget (- (Utilities|Array|Length _targets) 1))
    (Rendering|SetActorHiddenInGame (Utilities|Array|Get(acopy) _targets _currenttarget) true)))