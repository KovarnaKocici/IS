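; Pac-Man coin spawner that scatters BP_Coin actors over the navmesh within its Sphere radius when SpawnTargets is called; its own events are empty.
; Each pass snaps random navigable points to a 200-unit grid at fixed height and skips spawning if a coin overlaps.
; The random point is re-rolled per use, so checked and spawned positions can differ.
; The retry increment requires Targets >= NumTargets × 1000, so skips normally go unreplaced.
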(event EventBeginPlay)

(event Collision|EventActorBeginOverlap
  (params (OtherActor :type Actor%20Object%20Reference)))

(event EventTick
  (params (DeltaSeconds :type Float%20%28single-precision%29)))

(fn ConstructionScript)

(fn SpawnTargets
  (bind _returnvalue (Class|NavigationSystem|GetNavigationSystem))
  (bind _returnvalue_2 (Transformation|GetActorLocation))
  (bind _sphere (Variables|Default|GetSphere))
  (bind _returnvalue_3 (Components|Sphere|GetScaledSphereRadius _sphere))
  (bind _randomlocation (Class|NavigationSystem|GetRandomPointinNavigableRadius _returnvalue _returnvalue_2 _returnvalue_3))
  (bind _returnvalue_4 (Math|Float|%(Float) (.y _randomlocation) 2e+02))
  (bind _returnvalue_5 (Math|Float|%(Float) (.x _randomlocation) 2e+02))
  (bind _returnvalue_6 (- (.y _randomlocation) _returnvalue_4))
  (bind _returnvalue_7 (- (.x _randomlocation) _returnvalue_5))
  (bind _returnvalue_8 (Math|Vector|MakeVector _returnvalue_7 _returnvalue_6 2e+02))
  (Variables|Default|SetTargets (Variables|Default|GetNumTargets))
  (for _index (range 0 (Variables|Default|GetTargets))
    (bind _returnvalue_9 (Collision|SphereOverlapActors _returnvalue_8 1e+02 (Utilities|Array|MakeArray "ObjectTypeQuery2" "ObjectTypeQuery1") "/Game/Pacman/Blueprints/BP_Coin.BP_Coin_C"))
    (if _returnvalue_9
      (if (>= (Variables|Default|GetTargets) (* (Variables|Default|GetNumTargets) 1000))
        (Math|Integer|IncrementInt (Variables|Default|GetTargets)))
      (else
        (Game|SpawnActorfromClass "/Game/Pacman/Blueprints/BP_Coin.BP_Coin_C" (Math|Transform|MakeTransform _returnvalue_8 "0, 0, 0" "1,1,1") "AdjustIfPossibleButDontSpawnIfColliding" 0 0)))))